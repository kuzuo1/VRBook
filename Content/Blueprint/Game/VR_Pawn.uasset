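; VR_Pawn is the player pawn for VR, responsible for spawning the motion hands.
; On BeginPlay it spawns a BP_DefaultHand and a BP_RightHand actor with itself as owner, without storing either reference.
; RegisterHandsWithEachOther cross-links the left and right hand references when both are valid, but nothing in this graph calls it or sets those references.
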(event EventBeginPlay
  (Game|SpawnActorfromClass "/Game/Blueprint/Game/BP_Defaulthand.BP_DefaultHand_C" (Math|Transform|MakeTransform "0, 0, 0" "0, 0, 0" "1,1,1") "Undefined" self 0)
  (Game|SpawnActorfromClass "/Game/Blueprint/Game/BP_RightHand.BP_RightHand_C" (Math|Transform|MakeTransform "0, 0, 0" "0, 0, 0" "1,1,1") "Undefined" self 0))

(event Collision|EventActorBeginOverlap
  (params (OtherActor :type Actor%20Object%20Reference)))

(event EventTick
  (params (DeltaSeconds :type Float%20%28single-precision%29)))

(fn ConstructionScript)

(fn RegisterHandswithEachOther
  (if (and (Utilities|IsValid (Variables|Default|GetLeftHandBlueprint)) (Utilities|IsValid (Variables|Default|GetRightHandBlueprint)))
    (Variables|/Game/Blueprint/Game/BP_Defaulthand.BP_DefaultHand_C|SetOtherHandBlueprint (Variables|Default|GetLeftHandBlueprint) (Variables|Default|GetRightHandBlueprint))
    (Variables|/Game/Blueprint/Game/BP_Defaulthand.BP_DefaultHand_C|SetOtherHandBlueprint (Variables|Default|GetRightHandBlueprint) (Variables|Default|GetLeftHandBlueprint))))