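; BP_Defaulthand is a VR hand actor that represents the left or right hand of its owning VR_Pawn.
; On BeginPlay it registers itself on the pawn by its Hand setting, snap-attaches to the matching motion controller and has the pawn register the hands with each other.
; Registration also enables tick, which caches that side's trigger and grip axis values in TriggerAmount and GripAmount.
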(event EventBeginPlay
  (CallFunction|RegisterwithOwnerPawn))

(event EventTick
  (params (DeltaSeconds :type Float%20%28single-precision%29))
  (Variables|Default|SetTriggerAmount (Utilities|Select :Index (Variables|Default|GetHand) :Left (Input|AxisValues|GetMotionController(L)TriggerAxis) :Right (Input|AxisValues|GetMotionController(R)TriggerAxis) :AnyHand 0.0 :Pad 0.0 :ExternalCamera 0.0 :Gun 0.0 :Special_1 0.0 :Special_2 0.0 :Special_3 0.0 :Special_4 0.0 :Special_5 0.0 :Special_6 0.0 :Special_7 0.0 :Special_8 0.0 :Special_9 0.0 :Special_10 0.0 :Special_11 0.0))
  (Variables|Default|SetGripAmount (Utilities|Select :Index (Variables|Default|GetHand) :Left (Input|AxisValues|GetMotionController(L)GripAxis) :Right (Input|AxisValues|GetMotionController(R)GripAxis) :AnyHand 0.0 :Pad 0.0 :ExternalCamera 0.0 :Gun 0.0 :Special_1 0.0 :Special_2 0.0 :Special_3 0.0 :Special_4 0.0 :Special_5 0.0 :Special_6 0.0 :Special_7 0.0 :Special_8 0.0 :Special_9 0.0 :Special_10 0.0 :Special_11 0.0)))

(fn ConstructionScript)

(fn RegisterwithOwnerPawn
  (bind _asvr_pawn (Utilities|Casting|CastToVR_Pawn (Components|GetOwner)))
  (Variables|Default|SetPawn _asvr_pawn)
  (Actor|Tick|SetActorTickEnabled true)
  (switch Utilities|FlowControl|Switch|SwitchonEControllerHand (Variables|Default|GetHand)
    (:Left
      (Variables|/Game/Blueprint/Game/VR_Pawn.VR_Pawn_C|SetLeftHandBlueprint (Variables|Default|GetPawn) self)
      (bind _output_get (Variables|Default|SetMotionControllerComponent (Variables|/Game/Blueprint/Game/VR_Pawn.VR_Pawn_C|GetLeft_MotionController (Variables|Default|GetPawn))))
      (Transformation|AttachComponentToComponent _output_get "None" "SnapToTarget" "SnapToTarget" "SnapToTarget" false))
    (:Right
      (Variables|/Game/Blueprint/Game/VR_Pawn.VR_Pawn_C|SetRightHandBlueprint (Variables|Default|GetPawn) self)
      (bind _output_get_2 (Variables|Default|SetMotionControllerComponent (Variables|/Game/Blueprint/Game/VR_Pawn.VR_Pawn_C|GetRight_MotionController (Variables|Default|GetPawn))))
      (Transformation|AttachComponentToComponent _output_get_2 "None" "SnapToTarget" "SnapToTarget" "SnapToTarget" false)))
  (Default|RegisterHandswithEachOther (Variables|Default|GetPawn)))